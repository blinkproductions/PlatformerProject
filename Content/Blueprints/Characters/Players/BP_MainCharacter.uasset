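; BP_MainCharacter is the player character Blueprint, handling melee combat, weapon drawing and aim-down-sights.
; Attacking requires a drawn weapon and plays a montage, chaining combo hits by setting the next section when input lands in a "ComboWindow" section.
; Equip input toggles the weapon between hand and sheath sockets alongside a montage.
; Aiming switches rotation to controller-driven and scales spring arm length through a reversible timeline, with debug prints active.
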(event Custom|GenericAttack
  (bind _mesh (Variables|Character|GetMesh))
  (bind _mesh_2 (Variables|Character|GetMesh))
  (bind _mesh_3 (Variables|Character|GetMesh))
  (bind _returnvalue (Components|SkeletalMesh|GetAnimInstance _mesh_2))
  (bind _returnvalue_2 (Components|SkeletalMesh|GetAnimInstance _mesh))
  (bind _returnvalue_3 (Components|SkeletalMesh|GetAnimInstance _mesh_3))
  (bind _returnvalue_4 (Animation|Montage|GetCurrentActiveMontage _returnvalue_2))
  (if (not (Class|AnimInstance|IsAnyMontagePlaying (Components|SkeletalMesh|GetAnimInstance (Variables|Character|GetMesh))))
    (Variables|Default|SetbIsAttacking true)
    (Animation|Montage|PlayMontage (Variables|Character|GetMesh) "/Game/Assets/Characters/Player/Armed/Combat/MeleeAttackMontage.MeleeAttackMontage" 1.0 0.0 "Attack1"
      (:OnBlendOut
        (Variables|Default|SetbIsAttacking false)))
    (else
      ;[1 1 1] Check if the montage that is currently playing is the Attack1
      (if (Animation|Montage|MontageIsPlaying (Components|SkeletalMesh|GetAnimInstance (Variables|Character|GetMesh)) "/Game/Assets/Characters/Player/Armed/Combat/MeleeAttackMontage.MeleeAttackMontage")
        ;[1 1 1] Checks if we are inside a combo window
        (if (Utilities|String|Contains (Utilities|String|ToString(Name) (Animation|Montage|MontageGetCurrentSection _returnvalue (Animation|Montage|GetCurrentActiveMontage _returnvalue))) "ComboWindow")
          (Class|AnimInstance|MontageSetNextSection _returnvalue_2 (Animation|Montage|MontageGetCurrentSection _returnvalue_2 _returnvalue_4) (Utilities|String|StringToName (Utilities|String|Append "Attack" (Utilities|String|SelectString "2" "3" (Utilities|String|Contains (Utilities|String|ToString(Name) (Animation|Montage|MontageGetCurrentSection _returnvalue_3 (Animation|Montage|GetCurrentActiveMontage _returnvalue_3))) "1")))) _returnvalue_4))))))

(event EventBeginPlay)

(event EventTick
  (params (DeltaSeconds :type Float%20%28single-precision%29))
  (Development|PrintString (Utilities|String|ToString(Float) (Variables|/Script/Engine.SpringArmComponent|GetTargetArmLength (Variables|Default|GetSpringArm))) true true "(R=0.000000,G=0.660000,B=1.000000,A=1.000000)" 0.0))

(event Input|ActionEvents|InputActionAttack
  (params (Key :type Key%20Structure :default "None"))
  (:Pressed
    (if (Variables|Default|GetbIsWeaponDrawn)
      (CallFunction|GenericAttack))))

(event Input|ActionEvents|InputActionEquipWeapon1
  (params (Key :type Key%20Structure :default "None"))
  (bind _mesh (Variables|Character|GetMesh))
  (bind _equippedweapon1 (Variables|Default|GetEquippedWeapon1))
  (bind _mesh_2 (Variables|Character|GetMesh))
  (:Pressed
    (bind _output_get (Variables|Default|SetbIsWeaponDrawn (not (Variables|Default|GetbIsWeaponDrawn))))
    (if _output_get
      (Animation|Montage|PlayMontage _mesh_2 "/Game/Assets/Characters/Player/Armed/Combat/EquipWeapon.EquipWeapon" 2.0
        (:then
          (Utilities|FlowControl|Delay 0.1)
          (Transformation|AttachComponentToComponent _equippedweapon1 _mesh "WeaponSocket" "KeepWorld" "KeepWorld" "KeepWorld" true)))
      (else
        (Animation|Montage|PlayMontage _mesh_2 "/Game/Assets/Characters/Player/Armed/Combat/EquipWeapon.EquipWeapon" 2.0
          (:then
            (Utilities|FlowControl|Delay 0.01)
            (Transformation|AttachComponentToComponent _equippedweapon1 _mesh "WeaponSheath1" "KeepWorld" "KeepWorld" "KeepWorld" true)))))
    (Components|MoveComponentTo _equippedweapon1 "0, 0, 0" "0, 0, 0" false false 0.2 false)))

(event Input|ActionEvents|InputActionAimDownSights
  (params (Key :type Key%20Structure :default "None"))
  (bind _charactermovement (Variables|Character|GetCharacterMovement))
  (bind _charactermovement_2 (Variables|Character|GetCharacterMovement))
  (:Pressed
    (Variables|/Script/Engine.CharacterMovementComponent|SetbUseControllerDesiredRotation _charactermovement_2 true)
    (Variables|/Script/Engine.CharacterMovementComponent|SetbOrientRotationToMovement _charactermovement_2 false)
    (bind _delta (Timeline|ADSTimeline Play)
      (:Update
        (Development|PrintString (Utilities|String|ToString(Float) (* (Variables|Default|GetDefaultSpringArmLength) _delta)))
        (Variables|/Script/Engine.SpringArmComponent|SetTargetArmLength (Variables|Default|GetSpringArm) (* (Variables|Default|GetDefaultSpringArmLength) _delta)))))
  (:Released
    (Variables|/Script/Engine.CharacterMovementComponent|SetbUseControllerDesiredRotation _charactermovement false)
    (Variables|/Script/Engine.CharacterMovementComponent|SetbOrientRotationToMovement _charactermovement true)
    (Timeline|ADSTimeline Reverse)))

(fn ConstructionScript)